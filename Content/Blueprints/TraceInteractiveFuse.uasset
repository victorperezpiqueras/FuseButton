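; Trace-interactive cube that selects itself after being focused for a two-second "fuse", as in gaze-style dwell selection.
; Trace callbacks set Focused and Selected, recolor the cube by state, and move an arrow to the hit point.
; Tick turns the timer toward the player and counts focus time into a dynamic ring material's progress.
; On completion it calls TraceActivateDown itself with a synthesized hit; losing focus resets the timer.
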(event `self.ReceiveTick`
  (params (DeltaSeconds :type "Float (single-precision)"))
  (`self.updateTimerOrientation`)
  ;[1 1 1] check if object is focused
  (if (`self.focused`)
    ;[1 1 1] check if object is selected
    (if (`self.selected`)
      ;[1 1 1] if not focused or is already selected->reset time and timer
      (set `self.counted_time` 0.0 :!label _label)
      (`self.resetTimer`)
      (else
        ;[1 1 1] if object focused and not selected->count time and update timer
        (`SceneComponent.SetVisibility` (`self.Timer`) true false)
        (bind _output_get (`self.countTime` DeltaSeconds))
        (`self.updateTimer` _output_get)))
    (else
      (goto _label))))

(fn `countTime`
  (params (time :type "Float (double-precision)"))
  (returns (Output_Get :type "Float (double-precision)"))
  (bind _output_get (set `self.counted_time` (+ time (`self.counted_time`))))
  (return _output_get))

(fn `resetTimer`
  ;[1 1 1] Remove material, UIRing and visibility
  (set `self.UIRing` null)
  (`PrimitiveComponent.SetMaterial` (`self.Timer`) 0 null)
  (`SceneComponent.SetVisibility` (`self.Timer`) false false)
  (return))

(fn `TraceActivateDown`
  (params (Hit :type "HitResult Structure") (Instigator :type "Pawn Object Reference"))
  (returns (Return :type Boolean))
  ;[1 1 1] if activating cube component
  (if (== (`.HitComponent` (`GameplayStatics.BreakHitResult` Hit)) (`self.Cube`))
    (`MeshComponent.SetVectorParameterValueOnMaterials` (`self.Cube`) "Color" (0.0 1.0 0.0))
    ;[1 1 1] start selecting object
    (set `self.selected` true)
    (return false)))

(fn `TraceActivateUp`
  (params (Hit :type "HitResult Structure") (Instigator :type "Pawn Object Reference"))
  (returns (Return :type Boolean))
  ;[1 1 1] if activating cube component
  (if (== (`.HitComponent` (`GameplayStatics.BreakHitResult` Hit)) (`self.Cube`))
    (`MeshComponent.SetVectorParameterValueOnMaterials` (`self.Cube`) "Color" (1.0 1.0 0.0))
    ;[1 1 1] leave object selected
    (set `self.selected` false)
    (return false)))

(fn `TraceHitComponent`
  (params (Hit :type "HitResult Structure") (Component :type "PrimitiveComponent Object Reference"))
  (returns (Return :type Boolean))
  ;[1 1 1] if entering cube component
  (if (== Component (`self.Cube`))
    ;[1 1 1] set focused
    (set `self.focused` true)
    (`MeshComponent.SetVectorParameterValueOnMaterials` (`self.Cube`) "Color" (1.0 1.0 0.0))
    (return false)))

(fn `TraceHitObject`
  (params (Hit :type "HitResult Structure"))
  (returns (Return :type Boolean))
  (return false))

(fn `TraceLeaveComponent`
  (params (Hit :type "HitResult Structure") (Component :type "PrimitiveComponent Object Reference"))
  (returns (Return :type Boolean))
  ;[1 1 1] if leaving cube component
  (if (== Component (`self.Cube`))
    ;[1 1 1] set not focused nor selected
    (set `self.focused` false)
    (set `self.selected` false)
    (`MeshComponent.SetVectorParameterValueOnMaterials` (`self.Cube`) "Color" (1.0 1.0 1.0))
    (return false)))

(fn `TraceLeaveObject`
  (params (Hit :type "HitResult Structure"))
  (returns (Return :type Boolean))
  ;[1 1 1] set not focused nor selected
  (set `self.focused` false)
  (set `self.selected` false)
  (`MeshComponent.SetVectorParameterValueOnMaterials` (`self.Cube`) "Color" (1.0 1.0 1.0))
  (return false))

(fn `TraceMove`
  (params (Hit :type "HitResult Structure (by ref)"))
  (returns (Return :type Boolean))
  (bind (_bblockinghit _binitialoverlap _time _location _impactpoint _normal) (`GameplayStatics.BreakHitResult` Hit))
  (`SceneComponent.K2_SetWorldLocationAndRotation` (`self.Arrow`) _location (`KismetMathLibrary.MakeRotFromX` _normal) false false)
  (return false))

(fn `updateTimer`
  (params (time :type "Float (double-precision)"))
  ;[1 1 1] compare time with limit
  (if (>= time 2.0)
    ;[1 1 1] if focus time is completed -> reset timer and activate
    (`self.resetTimer`)
    (`self.TraceActivateDown` (`GameplayStatics.MakeHitResult` false false 0.0 (0.0 0.0 0.0) (0.0 0.0 0.0) (0.0 0.0 1.0) (0.0 0.0 1.0) null null (`self.Cube`)))
    (else
      ;[1 1 1] if focus time is not done yet -> update UIRing material
      (bind _returnvalue (`KismetMaterialLibrary.CreateDynamicMaterialInstance` "/Game/Materials/UIRing.UIRing"))
      (bind _output_get (set `self.UIRing` _returnvalue))
      (`MaterialInstanceDynamic.SetScalarParameterValue` _output_get "PercentComplete" (/ (`self.counted_time`) 2.0))
      (`PrimitiveComponent.SetMaterial` (`self.Timer`) 0 (`self.UIRing`)))))

(fn `updateTimerOrientation`
  ;[1 1 1] Rotate object towards user
  (`SceneComponent.K2_SetWorldRotation` (`self.Timer`) (`KismetMathLibrary.FindLookAtRotation` (`SceneComponent.K2_GetComponentLocation` (`self.Timer`)) (`self.K2_GetActorLocation` (`GameplayStatics.GetPlayerPawn` 0))) false false))

(fn `UserConstructionScript`)